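; Two-way teleporter actor that moves a Player-tagged actor between its BoxStart and BoxEnd trigger volumes.
; On overlap with either box, it disables the destination box's collision and sets the actor's location to that box.
; After a two-second delay, it restores query-only collision and prints a debug message, so arriving does not immediately bounce the player back.
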(event `self.BoxStart.OnComponentBeginOverlap`
  (params (OverlappedComponent :type "PrimitiveComponent Object Reference") (OtherActor :type "Actor Object Reference") (OtherComp :type "PrimitiveComponent Object Reference") (OtherBodyIndex :type Integer) (bFromSweep :type Boolean) (SweepResult :type "HitResult Structure (by ref)"))
  (if (`self.ActorHasTag` OtherActor "Player")
    (`PrimitiveComponent.SetCollisionEnabled` (`self.BoxEnd`) "NoCollision")
    (`self.K2_SetActorLocation` OtherActor (`SceneComponent.K2_GetComponentLocation` (`self.BoxEnd`)) false false)
    (`KismetSystemLibrary.Delay` 2.0)
    (`PrimitiveComponent.SetCollisionEnabled` (`self.BoxEnd`) "QueryOnly")
    (`KismetSystemLibrary.PrintString` "TELEPORTADO")))

(event `self.BoxEnd.OnComponentBeginOverlap`
  (params (OverlappedComponent :type "PrimitiveComponent Object Reference") (OtherActor :type "Actor Object Reference") (OtherComp :type "PrimitiveComponent Object Reference") (OtherBodyIndex :type Integer) (bFromSweep :type Boolean) (SweepResult :type "HitResult Structure (by ref)"))
  (if (`self.ActorHasTag` OtherActor "Player")
    (`PrimitiveComponent.SetCollisionEnabled` (`self.BoxStart`) "NoCollision")
    (`self.K2_SetActorLocation` OtherActor (`SceneComponent.K2_GetComponentLocation` (`self.BoxStart`)) false false)
    (`KismetSystemLibrary.Delay` 2.0)
    (`PrimitiveComponent.SetCollisionEnabled` (`self.BoxStart`) "QueryOnly")
    (`KismetSystemLibrary.PrintString` "TELEPORTADO")))

(fn `UserConstructionScript`)