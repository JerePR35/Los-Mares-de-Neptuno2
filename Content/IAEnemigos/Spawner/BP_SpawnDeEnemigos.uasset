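; Enemy spawner Blueprint that refills a tracked group of AI enemies at random points inside its Box bounds.
; RevisarEnemigos prunes invalid entries from the Enemigos array, then SpawnearEnemigos tops it up to ten whenever fewer than five remain.
; Nothing in this graph calls that check: BeginPlay and SpawnearTrigger are empty, and the looping timer and older delay-loop spawner are disconnected.
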(event `self.ReceiveBeginPlay`)

(event `RevisarEnemigos`
  (bind (_arrayindex _arrayelement) (`/Engine/EditorBlueprintResources/StandardMacros.ReverseForEachLoop` (`self.Enemigos`))
    (:`LoopBody`
      (`/Engine/EditorBlueprintResources/StandardMacros.IsValid` _arrayelement
        (:`Is Not Valid`
          (`KismetArrayLibrary.Array_Remove` (`self.Enemigos`) _arrayindex))))
    (:`Completed`
      (`self.SpawnearEnemigos`))))

(event `SpawnearEnemigos`
  (bind _returnvalue (`KismetArrayLibrary.Array_Length` (`self.Enemigos`)))
  (bind (_origin _boxextent) (`KismetSystemLibrary.GetComponentBounds` (`self.Box`)))
  (if (< _returnvalue 5)
    (for _ (range 1 (+ (- 10 _returnvalue) 1))
      (bind _returnvalue_2 (`AIBlueprintHelperLibrary.SpawnAIFromClass` "/Game/IAEnemigos/Actores/BP´_Enemigo_Child2.BP´_Enemigo_Child2_C" "/Game/IAEnemigos/BT_Enemigo.BT_Enemigo" (`KismetMathLibrary.RandomPointInBoundingBox` _origin _boxextent) (struct) false null))
      (`KismetArrayLibrary.Array_Add` (`self.Enemigos`) _returnvalue_2))))

(event `SpawnearTrigger`)

(fn `UserConstructionScript`)