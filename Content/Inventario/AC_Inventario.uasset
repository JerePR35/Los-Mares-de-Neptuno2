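; Player inventory component with nine item slots and a three-slot hotbar, driving the inventory and hotbar widgets.
; AgarrarObjetos adds pickups via name match or free slot, capping stacks and returning leftovers, though the match only accepts already-full stacks.
; IA_Inventario swaps inventory and hotbar views, toggling cursor and look input.
; Number inputs set the player's SKMSworrd mesh from the chosen hotbar slot, supplied through RefJugador.
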(event `self.ReceiveBeginPlay`
  (bind _returnvalue (`|CreateWidget` "/Game/Inventario/Widgets/WB_Inventario.WB_Inventario_C"))
  (set `self.WidgetInventario` _returnvalue)
  (bind _returnvalue_2 (`|CreateWidget` "/Game/ThirdPerson/Character/Personaje/UI/WB_UI.WB_UI_C"))
  (set `self.WB_Hotbar` _returnvalue_2)
  (`KismetArrayLibrary.Array_Resize` (`self.Objetos`) 9)
  (`KismetArrayLibrary.Array_Resize` (`self.Hotbar`) 3)
  (`/Game/Inventario/Widgets/WB_Inventario.Cargar inventario` (`self.WidgetInventario`) self)
  (`/Game/ThirdPerson/Character/Personaje/UI/WB_UI.CargarHotbar` (`self.WB_Hotbar`) self)
  (`UserWidget.AddToViewport` (`self.WB_Hotbar`) 0))

(event `EnhancedInput|/Game/Input/Actions/IA_Inventario`
  (params (ActionValue :type Boolean) (ElapsedSeconds :type "Float (double-precision)") (TriggeredSeconds :type "Float (double-precision)") (InputAction :type "InputAction Object Reference" :default "/Game/Input/Actions/IA_Inventario.IA_Inventario"))
  (:`Started`
    (if (`Widget.IsVisible` (`self.WidgetInventario`))
      (`self.Ocultar inventario`)
      (else
        (`self.Mostrar inventario`)))))

(event `EnhancedInput|/Game/Input/Actions/IA_Uno`
  (params (ActionValue :type Boolean) (ElapsedSeconds :type "Float (double-precision)") (TriggeredSeconds :type "Float (double-precision)") (InputAction :type "InputAction Object Reference" :default "/Game/Input/Actions/IA_Uno.IA_Uno"))
  (:`Started`
    (set `self.Slot Equipado` 0)
    (`self.Equipar Objeto` :!label _label)))

(event `EnhancedInput|/Game/Input/Actions/IA_Dos`
  (params (ActionValue :type Boolean) (ElapsedSeconds :type "Float (double-precision)") (TriggeredSeconds :type "Float (double-precision)") (InputAction :type "InputAction Object Reference" :default "/Game/Input/Actions/IA_Dos.IA_Dos"))
  (:`Started`
    (set `self.Slot Equipado` 1)
    (goto _label)))

(event `EnhancedInput|/Game/Input/Actions/IA_Tres`
  (params (ActionValue :type Boolean) (ElapsedSeconds :type "Float (double-precision)") (TriggeredSeconds :type "Float (double-precision)") (InputAction :type "InputAction Object Reference" :default "/Game/Input/Actions/IA_Tres.IA_Tres"))
  (:`Started`
    (set `self.Slot Equipado` 2)
    (goto _label)))

(fn `Agarrar objetos`
  (params (Objeto :type "/Game/Inventario/BS_Objeto Structure"))
  (returns (Sobro :type Integer))
  (locals (`Nuevo Objeto` :type "/Game/Inventario/BS_Objeto Structure"))
  (bind (_nuevo_objeto_name _nuevo_objeto_descripcion _nuevo_objeto_cantidad _nuevo_objeto_cantidadmax) (break `/Game/Inventario/BS_Objeto` (`local.Nuevo Objeto`)))
  (bind (_nuevo_objeto_name_2 _nuevo_objeto_descripcion_2 _nuevo_objeto_cantidad_2) (break `/Game/Inventario/BS_Objeto` (`local.Nuevo Objeto`)))
  (bind (_nuevo_objeto_name_3 _nuevo_objeto_descripcion_3 _nuevo_objeto_cantidad_3) (break `/Game/Inventario/BS_Objeto` (`local.Nuevo Objeto`)))
  (bind (_nuevo_objeto_name_4 _nuevo_objeto_descripcion_4 _nuevo_objeto_cantidad_4) (break `/Game/Inventario/BS_Objeto` (`local.Nuevo Objeto`)))
  (bind _nuevo_objeto (`local.Nuevo Objeto`))
  (bind _nuevo_objeto_2 (`local.Nuevo Objeto`))
  (bind (_name _descripcion _cantidad _cantidadmax _icono _mesh _esarma_ _peso _skmesh) (break `/Game/Inventario/BS_Objeto` _nuevo_objeto_2))
  (bind (_name_2 _descripcion_2 _cantidad_2 _cantidadmax_2 _icono_2 _mesh_2 _esarma__2 _peso_2 _skmesh_2) (break `/Game/Inventario/BS_Objeto` _nuevo_objeto))
  (set `local.Nuevo Objeto` Objeto)
  (if (> _nuevo_objeto_cantidadmax 1)
    (while (> _nuevo_objeto_cantidad_3 0)
      (bind _posicion_slot (`self.Buscar en el Inventario` (`local.Nuevo Objeto`)))
      (if (>= _posicion_slot 0)
        (bind _sobrante (`self.Agregar a Slot` _posicion_slot _nuevo_objeto_2))
        (set `local.Nuevo Objeto` (make `/Game/Inventario/BS_Objeto` _name _descripcion _sobrante _cantidadmax _icono _mesh _esarma_ _peso _skmesh))
        (else
          (bind _pos_slot_libre (`self.Buscar Slot Libre`))
          (if (>= _pos_slot_libre 0)
            (bind _sobrante_2 (`self.Agregar a Slot` _pos_slot_libre _nuevo_objeto))
            (set `local.Nuevo Objeto` (make `/Game/Inventario/BS_Objeto` _name_2 _descripcion_2 _sobrante_2 _cantidadmax_2 _icono_2 _mesh_2 _esarma__2 _peso_2 _skmesh_2))
            (else
              (return _nuevo_objeto_cantidad_2))))))
    (return 0)
    (else
      (bind _pos_slot_libre_2 (`self.Buscar Slot Libre`))
      (if (>= _pos_slot_libre_2 0)
        (`self.Agregar a Slot` _pos_slot_libre_2 (`local.Nuevo Objeto`))
        (else
          (return _nuevo_objeto_cantidad_4))))))

(fn `Agregar a Slot`
  (params (Slot :type Integer) (Objeto :type "/Game/Inventario/BS_Objeto Structure"))
  (returns (Sobrante :type Integer))
  (locals (`Pos Slot` :type Integer) (`Nuevo Objeto` :type "/Game/Inventario/BS_Objeto Structure") (`Objeto Almacenado` :type "/Game/Inventario/BS_Objeto Structure"))
  (bind (_objeto_almacenado_name _objeto_almacenado_descripcion _objeto_almacenado_cantidad) (break `/Game/Inventario/BS_Objeto` (`local.Objeto Almacenado`)))
  (bind (_nuevo_objeto_name _nuevo_objeto_descripcion _nuevo_objeto_cantidad _nuevo_objeto_cantidadmax _nuevo_objeto_icono _nuevo_objeto_mesh _nuevo_objeto_esarma_ _nuevo_objeto_peso _nuevo_objeto_skmesh) (break `/Game/Inventario/BS_Objeto` (`local.Nuevo Objeto`)))
  (bind (_nuevo_objeto_name_2 _nuevo_objeto_descripcion_2 _nuevo_objeto_cantidad_2 _nuevo_objeto_cantidadmax_2 _nuevo_objeto_icono_2 _nuevo_objeto_mesh_2 _nuevo_objeto_esarma__2 _nuevo_objeto_peso_2 _nuevo_objeto_skmesh_2) (break `/Game/Inventario/BS_Objeto` (`local.Nuevo Objeto`)))
  (bind _returnvalue (+ _objeto_almacenado_cantidad _nuevo_objeto_cantidad))
  (set `local.Pos Slot` Slot)
  (set `local.Nuevo Objeto` Objeto)
  (set `local.Objeto Almacenado` (`|GetArrayItem` (`self.Objetos`) (`local.Pos Slot`)))
  (if (> _returnvalue _nuevo_objeto_cantidadmax)
    (`KismetArrayLibrary.Array_Set` (`self.Objetos`) (`local.Pos Slot`) (make `/Game/Inventario/BS_Objeto` _nuevo_objeto_name_2 _nuevo_objeto_descripcion_2 _nuevo_objeto_cantidadmax_2 _nuevo_objeto_cantidadmax_2 _nuevo_objeto_icono_2 _nuevo_objeto_mesh_2 _nuevo_objeto_esarma__2 _nuevo_objeto_peso_2 _nuevo_objeto_skmesh_2))
    (`/Game/Inventario/Widgets/WB_Inventario.Cargar inventario` (`self.WidgetInventario`) self)
    (return (- _returnvalue _nuevo_objeto_cantidadmax_2))
    (else
      (`KismetArrayLibrary.Array_Set` (`self.Objetos`) (`local.Pos Slot`) (make `/Game/Inventario/BS_Objeto` _nuevo_objeto_name _nuevo_objeto_descripcion _returnvalue _nuevo_objeto_cantidadmax _nuevo_objeto_icono _nuevo_objeto_mesh _nuevo_objeto_esarma_ _nuevo_objeto_peso _nuevo_objeto_skmesh))
      (`/Game/Inventario/Widgets/WB_Inventario.Cargar inventario` (`self.WidgetInventario`) self)
      (return 0))))

(fn `Buscar en el Inventario`
  (params (`Objeto ` :type "/Game/Inventario/BS_Objeto Structure"))
  (returns (`Posicion slot` :type Integer))
  (locals (`Nuevo Objeto` :type "/Game/Inventario/BS_Objeto Structure"))
  (bind (_nuevo_objeto_name _nuevo_objeto_descripcion _nuevo_objeto_cantidad _nuevo_objeto_cantidadmax) (break `/Game/Inventario/BS_Objeto` (`local.Nuevo Objeto`)))
  (set `local.Nuevo Objeto` `Objeto `)
  (for (_array_element _array_index) (`self.Objetos`)
    (bind (_name _descripcion _cantidad) (break `/Game/Inventario/BS_Objeto` _array_element))
    (if (== _name _nuevo_objeto_name)
      (if (>= _cantidad _nuevo_objeto_cantidadmax)
        (return _array_index))))
  (return -1))

(fn `Buscar Slot Libre`
  (returns (`Pos Slot Libre` :type Integer))
  (for (_array_element _array_index) (`self.Objetos`)
    (if (== (`.Name_32_E03D889043EBDEBA074D60B1190F4CB5` (break `/Game/Inventario/BS_Objeto` _array_element)) "None")
      (return _array_index)))
  (return -1))

(fn `Equipar Objeto`
  (locals (Limpiar :type "SkeletalMesh Object Reference"))
  (bind _skm_sworrd (`self.SKM Sworrd`))
  (bind (_name _descripcion _cantidad _cantidadmax _icono _mesh _esarma_ _peso _skmesh) (break `/Game/Inventario/BS_Objeto` (`|GetArrayItem` (`self.Hotbar`) (`self.Slot Equipado`))))
  (`/Engine/EditorBlueprintResources/StandardMacros.IsValid` (`self.SKM Sworrd`)
    (:`Is Valid`
      (`/Engine/EditorBlueprintResources/StandardMacros.IsValid` _skmesh
        (:`Is Valid`
          (`SkeletalMeshComponent.SetSkeletalMeshAsset` _skm_sworrd _skmesh))
        (:`Is Not Valid`
          (`SkeletalMeshComponent.SetSkeletalMeshAsset` _skm_sworrd (`local.Limpiar`)))))))

(fn `Mostrar inventario`
  (bind _returnvalue (`GameplayStatics.GetPlayerController` 0))
  (set `PlayerController.bShowMouseCursor` true _returnvalue)
  (`WidgetBlueprintLibrary.SetInputMode_GameAndUIEx` _returnvalue null)
  (`UserWidget.AddToViewport` (`self.WidgetInventario`) 0)
  (`Controller.SetIgnoreLookInput` _returnvalue true)
  (`Widget.RemoveFromParent` (`self.WB_Hotbar`)))

(fn `Ocultar inventario`
  (bind _returnvalue (`GameplayStatics.GetPlayerController` 0))
  (set `PlayerController.bShowMouseCursor` false _returnvalue)
  (`Widget.RemoveFromParent` (`self.WidgetInventario`))
  (`WidgetBlueprintLibrary.SetInputMode_GameOnly` _returnvalue)
  (`Controller.ResetIgnoreLookInput` _returnvalue)
  (`UserWidget.AddToViewport` (`self.WB_Hotbar`) 0)
  (`/Game/ThirdPerson/Character/Personaje/UI/WB_UI.CargarHotbar` (`self.WB_Hotbar`) self))

(fn `Ref Jugador`
  (params (`Ref Jugador` :type "/Game/ThirdPerson/Character/Personaje/BP_ThirdPersonCharacter Object Reference"))
  (bind _output_get (set `self.Ref Player` `Ref Jugador`))
  (set `self.SKM Sworrd` (`/Game/ThirdPerson/Character/Personaje/BP_ThirdPersonCharacter.SKM_Sworrd` _output_get)))