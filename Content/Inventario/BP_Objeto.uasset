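; BP_Objeto is a world item actor that the player can pick up into their inventory.
; The construction script looks up its ID in DT_Objeto, then applies the row's mesh, enables physics and sets mass scale from the item's weight.
; On MensajeInteractuar it passes its item struct to the player's ACInventario.
; A positive returned count becomes the item's remaining quantity; otherwise the actor destroys itself.
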(event `/Game/Input/Actions/BPI_Interaccion.Mensaje interactuar`
  (params (`Ref Jugador` :type "/Game/ThirdPerson/Character/Personaje/BP_ThirdPersonCharacter Object Reference"))
  (bind (_objeto_name _objeto_descripcion _objeto_cantidad _objeto_cantidadmax _objeto_icono _objeto_mesh _objeto_esarma_ _objeto_peso _objeto_skmesh) (break `/Game/Inventario/BS_Objeto` (`self.Objeto`)))
  (bind _sobro (`/Game/Inventario/AC_Inventario.Agarrar objetos` (`/Game/ThirdPerson/Character/Personaje/BP_ThirdPersonCharacter.AC_Inventario` `Ref Jugador`) (`self.Objeto`)))
  (if (> _sobro 0)
    (set `self.Objeto` (make `/Game/Inventario/BS_Objeto` _objeto_name _objeto_descripcion _sobro _objeto_cantidadmax _objeto_icono _objeto_mesh _objeto_esarma_ _objeto_peso _objeto_skmesh))
    (else
      (`self.K2_DestroyActor`))))

(fn `UserConstructionScript`
  (bind _staticmesh (`self.StaticMesh`))
  (bind (_objeto_name _objeto_descripcion _objeto_cantidad _objeto_cantidadmax _objeto_icono _objeto_mesh _objeto_esarma_ _objeto_peso) (break `/Game/Inventario/BS_Objeto` (`self.Objeto`)))
  (bind _returnvalue (`|GetDataTableRow` "/Game/Inventario/DT_Objeto.DT_Objeto" (`self.ID`))
    (:`then`
      (set `self.Objeto` _returnvalue)
      (`StaticMeshComponent.SetStaticMesh` _staticmesh _objeto_mesh)
      (`PrimitiveComponent.SetSimulatePhysics` _staticmesh true)
      (`PrimitiveComponent.SetMassScale` _staticmesh "None" _objeto_peso))))